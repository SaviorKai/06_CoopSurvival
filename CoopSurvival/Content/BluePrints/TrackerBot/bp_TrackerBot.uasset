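; TrackerBot Blueprint, whose only live logic scales its audio volume with its movement speed.
; Tick maps velocity length to a clamped volume multiplier on AudioComp, so the bot gets louder as it moves faster.
; Disconnected example nodes show a synchronous navigation path to the player drawn with debug spheres, plus simple AI moves to a location or the player, but none of them run.
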(event `self.ReceiveBeginPlay`)

(event `self.ReceiveTick`
  (params (DeltaSeconds :type "Float (single-precision)"))
  (`AudioComponent.SetVolumeMultiplier` (`self.AudioComp`) (`KismetMathLibrary.MapRangeClamped` (`KismetMathLibrary.VSize` (`self.GetVelocity`)) 10.0 1000.0 0.1 2.0)))

(fn `UserConstructionScript`)