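; Grenade projectile Blueprint that explodes after a short fixed fuse starting at BeginPlay.
; Explode spawns an explosion particle effect, then applies radial damage using BaseDamage from the owning SGWeapon and the grenade's DamageRadius, then destroys the actor.
; If the owner is not an SGWeapon, execution stops after the effect, so no damage or destruction occurs.
; A debug sphere for the radius is left disconnected.
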(event `self.ReceiveBeginPlay`
  ;[1 1 1] Explode
  (`KismetSystemLibrary.Delay` 1.0)
  (`self.Explode`))

(event `Explode`
  ;[1 1 1] Explode
  (`GameplayStatics.SpawnEmitterAtLocation` "/Game/Weapons/WeaponEffects/Explosion/P_Explosion.P_Explosion" (`self.K2_GetActorLocation`))
  (bind _assgweapon (cast `SGWeapon` (`self.GetOwner`)))
  (`GameplayStatics.ApplyRadialDamage` :`BaseDamage` (`SGWeapon.BaseDamage` _assgweapon) :`Origin` (`self.K2_GetActorLocation`) :`DamageRadius` (`self.Damage Radius`) :`DamageCauser` self :`InstigatedByController` (`self.GetInstigatorController`))
  (`self.K2_DestroyActor`))

(fn `UserConstructionScript`)