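; Super speed power-up that temporarily doubles the walk speed of the first player's pawn.
; On activation it hides its mesh and child light through visibility propagation, then sets MaxWalkSpeed to twice the movement component's current GetMaxSpeed.
; On expiry it sets MaxWalkSpeed to half of GetMaxSpeed and destroys itself.
; Both events print the resulting speed, and the timing that triggers them lives outside these graphs.
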(event `self.OnActivated`
  (bind _returnvalue (`self.GetComponentByClass` (`GameplayStatics.GetPlayerPawn` 0) "/Script/Engine.CharacterMovementComponent"))
  ;[1 1 1] Because light is a child, light is also hidden because of Propagate to children.
  (`SceneComponent.SetVisibility` (`self.StaticMesh`) false true)
  (bind _output_get (set `CharacterMovementComponent.MaxWalkSpeed` (* (`MovementComponent.GetMaxSpeed` _returnvalue) 2.0) _returnvalue))
  (`KismetSystemLibrary.PrintString` (`KismetStringLibrary.Conv_DoubleToString` _output_get)))

(event `self.OnExpired`
  (bind _returnvalue (`self.GetComponentByClass` (`GameplayStatics.GetPlayerPawn` 0) "/Script/Engine.CharacterMovementComponent"))
  (bind _output_get (set `CharacterMovementComponent.MaxWalkSpeed` (/ (`MovementComponent.GetMaxSpeed` _returnvalue) 2.0) _returnvalue))
  (`self.K2_DestroyActor`)
  (`KismetSystemLibrary.PrintString` (`KismetStringLibrary.Conv_DoubleToString` _output_get)))

(fn `UserConstructionScript`)